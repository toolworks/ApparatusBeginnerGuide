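; BP_Mechanism is an ECS-style mechanism that runs movement and falling for subjects built from details, using two mechanics each Tick.
; The movement mechanic offsets Movable/Moving actors locally by direction and speed, then disables the Moving detail; Up is boosted and disables OnFloor, while Down has no offset.
; The falling mechanic, filtered on Fallable and OnFloor, re-adds OnFloor when Bottom overlaps actors, otherwise lowers the actor at constant speed.
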(event EventTick
  (params (DeltaSeconds :type Float%20%28single-precision%29))
  (Variables|Default|SetGlobalDelta DeltaSeconds)
  (Utilities|FlowControl|Sequence
    (:then_0
      (bind (_subject _subjective _detail_0 _detail_1) (|Mechanic "/Game/Details/D_Movable.D_Movable_C" "/Game/Details/D_Moving.D_Moving_C")
        (:EvaluationBody
          (Variables|Default|SetTempMoving _detail_1)
          (Transformation|AddActorLocalOffset (Class|ApparatusFunctionLibrary|GetSubjectiveActor _subjective) (Utilities|Select :Index (Variables|/Game/Details/D_Moving.D_Moving_C|GetDirection _detail_1) :None "0, 0, 0" :Left (Math|Vector|MakeVector 0.0 (* (Variables|/Game/Details/D_Movable.D_Movable_C|GetSpeed _detail_0) (Variables|Default|GetGlobalDelta)) 0.0) :Right (Math|Vector|MakeVector 0.0 (* -1 (* (Variables|/Game/Details/D_Movable.D_Movable_C|GetSpeed _detail_0) (Variables|Default|GetGlobalDelta))) 0.0) :Up (Math|Vector|MakeVector 0.0 0.0 (* 10 (* (Variables|/Game/Details/D_Movable.D_Movable_C|GetSpeed _detail_0) (Variables|Default|GetGlobalDelta)))) :Down "0, 0, 0") false false)
          (Variables|/Script/ApparatusRuntime.Detail|SetbEnabled (Variables|Default|GetTempMoving) false)
          (if (Utilities|Enum|Equal(Enum) "Up" (Variables|/Game/Details/D_Moving.D_Moving_C|GetDirection _detail_1))
            (Class|ApparatusFunctionLibrary|DisableSubjectiveDetail _subjective "/Game/Details/D_OnFloor.D_OnFloor_C" true)))))
    (:then_1
      (bind (_subject_2 _subjective_2 _detail_0_2) (|Mechanic "/Game/Details/D_Fallable.D_Fallable_C" "/Game/Details/D_OnFloor.D_OnFloor_C")
        (:EvaluationBody
          (Variables|Default|SetTempSubjective _subjective_2)
          (if (> (Utilities|Array|Length (Collision|GetOverlappingActors (Variables|/Game/Details/D_Fallable.D_Fallable_C|GetBottom _detail_0_2) "/Script/Engine.Actor" :!class /Script/Engine.PrimitiveComponent)) 0)
            (Class|ApparatusFunctionLibrary|AddSubjectiveDetail (Variables|Default|GetTempSubjective) "/Game/Details/D_OnFloor.D_OnFloor_C" true)
            (else
              (Transformation|AddActorWorldOffset (Class|ApparatusFunctionLibrary|GetSubjectiveActor (Variables|Default|GetTempSubjective)) (Math|Vector|MakeVector 0.0 0.0 (* -100 (Variables|Default|GetGlobalDelta)))))))))))

(fn ConstructionScript)