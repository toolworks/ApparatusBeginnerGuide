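; Main menu game mode that animates swaying actors and sets up the player's touch interface.
; On BeginPlay it calls ActivateTouchInterface on the first player controller with no interface specified.
; Each Tick runs an ECS-style mechanic over subjectives with the D_Swaying detail, setting each valid actor's rotation from the detail's GetNextRotator using delta time.
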(event EventBeginPlay
  (Class|PlayerController|ActivateTouchInterface (Game|GetPlayerController 0)))

(event EventTick
  (params (DeltaSeconds :type Float%20%28single-precision%29))
  (Variables|Default|SetDelta%20Seconds DeltaSeconds)
  (Utilities|FlowControl|Sequence
    (:then_0
      (bind (_subject _subjective _detail_0) (|Mechanic "/Game/MainMenu/D_Swaying.D_Swaying_C")
        (:Operate
          (Utilities|IsValid (Class|ApparatusFunctionLibrary|GetSubjectiveActor _subjective)
            (:Is%20Valid
              (Transformation|SetActorRotation (Class|ApparatusFunctionLibrary|GetSubjectiveActor _subjective) (Default|GetNextRotator _detail_0 (Variables|Default|GetDelta%20Seconds))))))))))

(fn ConstructionScript)