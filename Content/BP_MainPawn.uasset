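; Player pawn that turns left, right and jump input into movement data on a subjective actor, using Apparatus-style ECS details.
; Each press adds or reuses a disabled D_Moving detail on SubjectiveActor and sets its Direction to left, right or up.
; On BeginPlay it assigns Box as the Bottom of the existing D_Fallable detail.
; The graph only writes this data and applies no movement itself.
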(event EventBeginPlay
  (Variables|/Game/Details/D_Fallable.D_Fallable_C|SetBottom (Class|ApparatusFunctionLibrary|FindSubjectiveDetail (Variables|Default|GetSubjectiveActor) "/Game/Details/D_Fallable.D_Fallable_C" false) (Variables|Default|GetBox)))

(event Input|ActionEvents|InputActionLeftMoveInput
  (params (Key :type Key%20Structure :default "None"))
  (:Pressed
    (bind _returnvalue (Class|ApparatusFunctionLibrary|AddSubjectiveDetail (Variables|Default|GetSubjectiveActor) "/Game/Details/D_Moving.D_Moving_C" true))
    (Variables|/Game/Details/D_Moving.D_Moving_C|SetDirection _returnvalue "Left")))

(event Input|ActionEvents|InputActionRightMoveInput
  (params (Key :type Key%20Structure :default "None"))
  (:Pressed
    (bind _returnvalue (Class|ApparatusFunctionLibrary|AddSubjectiveDetail (Variables|Default|GetSubjectiveActor) "/Game/Details/D_Moving.D_Moving_C" true))
    (Variables|/Game/Details/D_Moving.D_Moving_C|SetDirection _returnvalue "Right")))

(event Input|ActionEvents|InputActionJumpMoveInput
  (params (Key :type Key%20Structure :default "None"))
  (:Pressed
    (bind _returnvalue (Class|ApparatusFunctionLibrary|AddSubjectiveDetail (Variables|Default|GetSubjectiveActor) "/Game/Details/D_Moving.D_Moving_C" true))
    (Variables|/Game/Details/D_Moving.D_Moving_C|SetDirection _returnvalue "Up")))

(fn ConstructionScript)